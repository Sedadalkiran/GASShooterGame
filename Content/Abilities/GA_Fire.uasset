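; Gameplay ability that fires a hitscan rifle shot, playing a hip-fire montage and ending when it completes or is interrupted.
; The locally controlled character starts weapon targeting, with PerformLocalTargeting line-tracing on the Camera channel from the eye viewpoint.
; When target data is ready, it executes the Fire gameplay cue from the hit result and applies GE_Damage only with authority.
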(event `self.K2_ActivateAbilityFromEvent`
  (params (EventData :type "GameplayEventData Structure (by ref)"))
  (`AbilityTask_PlayMontageAndWait.CreatePlayMontageAndWaitProxy` "None" "/Game/Characters/Mannequins/Animations/AnimStarterPack/Fire_Rifle_Hip_Retargeted_Montage.Fire_Rifle_Hip_Retargeted_Montage"
    (:`then`
      (bind _ascharacter (cast `Character` (`self.GetAvatarActorFromActorInfo`)))
      (if (`Pawn.IsLocallyControlled` _ascharacter)
        (`self.StartWeaponTargeting`)))
    (:`OnCompleted`
      (`self.K2_EndAbility` :!label _label))
    (:`OnInterrupted`
      (goto _label))
    (:`OnCancelled`
      (goto _label))))

(event `self.OnWeaponTargetDataReady`
  (params (TargetData :type "GameplayAbilityTargetDataHandle Structure (by ref)"))
  (`self.K2_ExecuteGameplayCueWithParams` (struct :`TagName` "GameplayCue.Fire") (`GameplayCueFunctionLibrary.MakeGameplayCueParametersFromHitResult` (`AbilitySystemBlueprintLibrary.GetHitResultFromTargetData` TargetData)))
  (`self.K2_HasAuthority`
    (:`True`
      (`self.BP_ApplyGameplayEffectToTarget` TargetData "/Game/Abilities/GE_Damage.GE_Damage_C"))))

(fn `PerformLocalTargeting`
  (returns (OutHits :type "HitResult Structure"))
  (bind _ascharacter (cast `Character` (`self.GetAvatarActorFromActorInfo`))
    (:`then`
      (bind (_outlocation _outrotation) (`Actor.GetActorEyesViewPoint` _ascharacter))
      (bind _outhit (`KismetSystemLibrary.LineTraceSingle` _outlocation (+ _outlocation (* (`KismetMathLibrary.Conv_RotatorToVector` _outrotation) 10000.0)) "TraceTypeQuery2" false (`|MakeArray` _ascharacter :!type "Actor Object Reference")))
      (return _outhit))
    (:`CastFailed`
      (return))))